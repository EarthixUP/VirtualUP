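; BreakableCoffeeMug is a destructible coffee mug actor that reacts to being shattered.
; When its destructible mesh component fractures, a counter ensures only the first break plays a quiet glass-breaking sound at the hit point.
; After a short delay the actor destroys itself, then sets IsCoffeeMugBroken on the VirtualUPGameInstance to record the break.
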(event OnComponentFracture(CoffeCup_DM)
  (params (HitPoint :type Vector%20%28by%20ref%29 :default "0, 0, 0") (HitDirection :type Vector%20%28by%20ref%29 :default "0, 0, 0"))
  (bind _result (Math|Integer|IncrementInt (Variables|Default|GetTimesBroken))
    (:%20%20
      (Variables|Default|SetTimesBroken _result)
      (if (== (Variables|Default|GetTimesBroken) 1)
        (Audio|PlaySoundatLocation "/Game/StarterContent/Audio/Glass_Breaking_Cue.Glass_Breaking_Cue" HitPoint "0, 0, 0" 0.01 1.0 0.0 0 0 0)
        (Utilities|FlowControl|Delay 4.0)
        (Actor|DestroyActor)
        (bind _asvirtual_upgame_instance (Utilities|Casting|CastToVirtualUPGameInstance (Game|GetGameInstance)))
        (Variables|/Game/GameModes/VirtualUPGameInstance.VirtualUPGameInstance_C|SetIsCoffeeMugBroken _asvirtual_upgame_instance true)))))

(event EventBeginPlay)

(event Collision|EventActorBeginOverlap
  (params (OtherActor :type Actor%20Object%20Reference)))

(event EventTick
  (params (DeltaSeconds :type Float%20%28single-precision%29)))

(fn ConstructionScript)