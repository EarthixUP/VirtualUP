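; Level actor that spawns toys: a breakable coffee mug and a smiley spray, each placed at its own arrow component.
; Both spawn on BeginPlay, and the mug is kept as the current cup.
; Tick polls the IsCoffeeMugBroken flag on the game instance, spawns a replacement mug when it is set, then clears the flag.
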(event EventBeginPlay
  (CallFunction|SpawnSmileySpray)
  (bind _newparam (CallFunction|SpawnCoffeeCup))
  (Variables|Default|SetCurrentCup _newparam))

(event Collision|EventActorBeginOverlap
  (params (OtherActor :type Actor%20Object%20Reference)))

(event EventTick
  (params (DeltaSeconds :type Float%20%28single-precision%29))
  (bind _asvirtual_upgame_instance (Utilities|Casting|CastToVirtualUPGameInstance (Game|GetGameInstance)))
  (if (Variables|/Game/GameModes/VirtualUPGameInstance.VirtualUPGameInstance_C|GetIsCoffeeMugBroken _asvirtual_upgame_instance)
    (bind _newparam (CallFunction|SpawnCoffeeCup))
    (Variables|Default|SetCurrentCup _newparam)
    (Variables|/Game/GameModes/VirtualUPGameInstance.VirtualUPGameInstance_C|SetIsCoffeeMugBroken _asvirtual_upgame_instance false)))

(fn ConstructionScript)

(fn SpawnCoffeeCup
  (bind _returnvalue (Game|SpawnActorfromClass "/Game/LevelBluePrints/Blueprints/BreakableCoffeeMug.BreakableCoffeeMug_C" (Transformation|GetWorldTransform (Variables|Default|GetArrow)) "Undefined" 0 0))
  (return _returnvalue))

(fn SpawnSmileySpray
  (bind _returnvalue (Game|SpawnActorfromClass "/Game/LevelBluePrints/Blueprints/SmileySpray.SmileySpray_C" (Transformation|GetWorldTransform (Variables|Default|GetArrow1)) "Undefined" 0 0))
  (return _returnvalue))