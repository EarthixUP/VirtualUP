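; FunModeBlock is an actor that toggles Scavenger Hunt mode on and off.
; A MASTERCLICK event or a Pawn overlapping the actor runs the same toggle logic.
; It flips IsGameModeOn on VirtualUPGameInstance, then updates the Square's red or green material and the TextRender label to show the new state.
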(event EventBeginPlay)

(event Collision|EventActorBeginOverlap
  (params (OtherActor :type Actor%20Object%20Reference))
  (bind _textrender (Variables|Default|GetTextRender))
  (Utilities|Casting|CastToPawn OtherActor)
  (bind _asvirtual_upgame_instance (Utilities|Casting|CastToVirtualUPGameInstance (Game|GetGameInstance)))
  (if (Variables|/Game/GameModes/VirtualUPGameInstance.VirtualUPGameInstance_C|GetisGameModeOn _asvirtual_upgame_instance)
    (Variables|/Game/GameModes/VirtualUPGameInstance.VirtualUPGameInstance_C|SetisGameModeOn _asvirtual_upgame_instance false)
    (Rendering|Material|SetMaterial (Variables|Default|Getsquare) 0 "/Game/PhotoR_Backgrounds/Meshes/template_red.template_red")
    (Rendering|Components|TextRender|SetText _textrender (Utilities|Text|ToText(String) (Utilities|String|MakeLiteralString "Scavenger Hunt: Disabled")))
    (else
      (Variables|/Game/GameModes/VirtualUPGameInstance.VirtualUPGameInstance_C|SetisGameModeOn _asvirtual_upgame_instance true)
      (Rendering|Material|SetMaterial (Variables|Default|Getsquare) 0 "/Game/Materials/GreenMaterial.GreenMaterial")
      (Rendering|Components|TextRender|SetText _textrender (Utilities|Text|ToText(String) (Utilities|String|MakeLiteralString "Scavenger Hunt: Enabled"))))))

(event EventTick
  (params (DeltaSeconds :type Float%20%28single-precision%29)))

(event EventMASTERCLICK
  (bind _textrender (Variables|Default|GetTextRender))
  (bind _asvirtual_upgame_instance (Utilities|Casting|CastToVirtualUPGameInstance (Game|GetGameInstance)))
  (if (Variables|/Game/GameModes/VirtualUPGameInstance.VirtualUPGameInstance_C|GetisGameModeOn _asvirtual_upgame_instance)
    (Variables|/Game/GameModes/VirtualUPGameInstance.VirtualUPGameInstance_C|SetisGameModeOn _asvirtual_upgame_instance false)
    (Rendering|Material|SetMaterial (Variables|Default|Getsquare) 0 "/Game/PhotoR_Backgrounds/Meshes/template_red.template_red")
    (Rendering|Components|TextRender|SetText _textrender (Utilities|Text|ToText(String) (Utilities|String|MakeLiteralString "Scavenger Hunt: Disabled")))
    (else
      (Variables|/Game/GameModes/VirtualUPGameInstance.VirtualUPGameInstance_C|SetisGameModeOn _asvirtual_upgame_instance true)
      (Rendering|Material|SetMaterial (Variables|Default|Getsquare) 0 "/Game/Materials/GreenMaterial.GreenMaterial")
      (Rendering|Components|TextRender|SetText _textrender (Utilities|Text|ToText(String) (Utilities|String|MakeLiteralString "Scavenger Hunt: Enabled"))))))

(fn ConstructionScript)