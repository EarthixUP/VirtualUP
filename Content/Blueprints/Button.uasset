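; Gaze button that activates after being looked at for a set delay.
; Looked and Unlooked events set a focus flag, and Tick accumulates a dwell timer while focused, setting Activated once it reaches the delay.
; When focus is lost, Activated clears immediately and the timer drains back toward zero at the same rate instead of resetting.
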(event Custom|Looked
  (Variables|Default|SetFocused true))

(event Custom|Unlooked
  (Variables|Default|SetFocused false))

(event EventTick
  (params (DeltaSeconds :type Float%20%28single-precision%29))
  (bind _delay (Variables|Default|GetDelay))
  (if (Variables|Default|GetFocused)
    (if (>= (Variables|Default|GetCurrDelay) _delay)
      (Variables|Default|SetCurrDelay _delay)
      (Variables|Default|SetActivated true)
      (else
        (Variables|Default|SetCurrDelay (+ (Variables|Default|GetCurrDelay) DeltaSeconds))))
    (else
      (if (<= (Variables|Default|GetCurrDelay) 0.0)
        (Variables|Default|SetCurrDelay 0.0)
        (else
          (Variables|Default|SetCurrDelay (- (Variables|Default|GetCurrDelay) DeltaSeconds))))
      (Variables|Default|SetActivated false))))

(fn ConstructionScript)